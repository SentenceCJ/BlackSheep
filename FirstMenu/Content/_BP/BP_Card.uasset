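; BP_Card is a card Blueprint that displays a number and can rotate between two states.
; The rotatecard and ReverseCardRotation events play a timeline forward or in reverse to drive the Cube's relative yaw, and set the Rotated flag.
; CardNumberShow writes CardNumber to the TextRender and also runs from the construction script, so the number is set when the actor is constructed.
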(event Custom|rotatecard
  (Variables|Default|SetbRotated true)
  (bind _rotation (Timeline|RotateAnim PlayFromStart)
    (:Update
      (Transformation|SetRelativeRotation (Variables|Default|GetCube) (Math|Rotator|MakeRotator 0.0 0.0 _rotation) false false))))

(event Custom|CardNumberShow
  (Rendering|Components|TextRender|SetText (Variables|Default|GetTextRender) (Utilities|Text|ToText(Integer) (Variables|Default|GetCardNumber))))

(event Custom|ReverseCardRotation
  (Variables|Default|SetbRotated false)
  (bind _rotation (Timeline|RotateAnim ReverseFromEnd)
    (:Update
      (Transformation|SetRelativeRotation (Variables|Default|GetCube) (Math|Rotator|MakeRotator 0.0 0.0 _rotation) false false))))

(fn ConstructionScript
  (CallFunction|CardNumberShow))