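; Player controller for a Simon-style memory game where the player picks cubes in a set order.
; Interact line-traces from the mouse, flashes the hit SimonCube's colour for a second, then compares it to the current entry in CubeColor_Manager's CubeOrder.
; A match advances CubeOrderIndex and shows WeLoveSimonScreen once the sequence is complete; a mismatch shows GameOver.
; The trace leaves persistent debug drawing on.
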(event Input|ActionEvents|InputActionInteract
  (params (Key :type Key%20Structure :default "None"))
  (bind (_worldlocation _worlddirection) (Game|Player|ConvertMouseLocationToWorldSpace))
  (bind _cubeorderindex (Variables|Default|GetcubeOrderIndex))
  (:Pressed
    (bind (_outhit _returnvalue) (Collision|LineTraceByChannel _worldlocation (+ _worldlocation (* _worlddirection 1.5e+03)) "TraceTypeQuery1" false 0 "Persistent"))
    (if _returnvalue
      (bind _assimon_cube (Utilities|Casting|CastToSimonCube (.HitActor (Collision|BreakHitResult _outhit))))
      (Default|ChangeColour _assimon_cube)
      (Utilities|FlowControl|Delay 1.0)
      (Default|ResetColour _assimon_cube)
      (bind _returnvalue_2 (Actor|GetActorOfClass "/Game/_BP/_Simon/CubeColor_Manager.CubeColor_Manager_C"))
      (if (== (Utilities|Array|Get(acopy) (Variables|/Game/_BP/_Simon/CubeColor_Manager.CubeColor_Manager_C|GetcubeOrder _returnvalue_2) (Variables|Default|GetcubeOrderIndex)) (.HitActor (Collision|BreakHitResult _outhit)))
        (Math|Integer|IncrementInt _cubeorderindex
          (:%20%20
            (if (>= _cubeorderindex (Utilities|Array|Length (Variables|/Game/_BP/_Simon/CubeColor_Manager.CubeColor_Manager_C|GetcubeOrder _returnvalue_2)))
              (bind _returnvalue_3 (UserInterface|CreateWidget "/Game/_Widgets/WeLoveSimonScreen.WeLoveSimonScreen_C"))
              (UserInterface|Viewport|AddtoViewport _returnvalue_3 0))))
        (else
          (bind _returnvalue_4 (UserInterface|CreateWidget "/Game/_Widgets/GameOver.GameOver_C"))
          (UserInterface|Viewport|AddtoViewport _returnvalue_4 0))))))

(fn ConstructionScript)