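; BP_Player is the player Blueprint that shows the HUD and runs the game's countdown to game over.
; On BeginPlay it creates WBP_HUD and adds it to the viewport.
; Each Tick subtracts delta time from the Timer stored in BP_GameInstance.
; When the timer reaches zero, it displays the GameOver widget and pauses the game.
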(event EventBeginPlay
  (bind _returnvalue (UserInterface|CreateWidget "/Game/_Widgets/WBP_HUD.WBP_HUD_C"))
  (UserInterface|Viewport|AddtoViewport _returnvalue 0))

(event EventTick
  (params (DeltaSeconds :type Float%20%28single-precision%29))
  (bind _asbp_game_instance (Utilities|Casting|CastToBP_GameInstance (Game|GetGameInstance)))
  (Variables|/Game/_BP/BP_GameInstance.BP_GameInstance_C|Settimer _asbp_game_instance (- (Variables|/Game/_BP/BP_GameInstance.BP_GameInstance_C|Gettimer _asbp_game_instance) DeltaSeconds))
  (if (<= (Variables|/Game/_BP/BP_GameInstance.BP_GameInstance_C|Gettimer _asbp_game_instance) 0.0)
    (bind _returnvalue (UserInterface|CreateWidget "/Game/_Widgets/GameOver.GameOver_C" (Game|GetPlayerController 0)))
    (UserInterface|Viewport|AddtoViewport _returnvalue 0)
    (Game|SetGamePaused true)))

(fn ConstructionScript)