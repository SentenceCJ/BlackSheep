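; Player controller for a spot-the-difference game that handles clicks on the hidden differences.
; On Interact, it deprojects the mouse position and runs a Visibility line trace into the world.
; Hitting an unfound DifferenceTick calls its ShowDiff, while an already found one is ignored.
; Hitting any other actor opens the GameOver widget and pauses the game; a trace that hits nothing does nothing.
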(event Input|ActionEvents|InputActionInteract
  (params (Key :type Key%20Structure :default "None"))
  (bind (_worldlocation _worlddirection) (Game|Player|ConvertMouseLocationToWorldSpace))
  (:Pressed
    (bind (_outhit _returnvalue) (Collision|LineTraceByChannel _worldlocation (+ _worldlocation (* _worlddirection 1.5e+03)) "TraceTypeQuery1" false 0 "None"))
    (if _returnvalue
      (bind _asdifference_tick (Utilities|Casting|CastToDifferenceTick (.HitActor (Collision|BreakHitResult _outhit)))
        (:then
          (if (not (Variables|/Game/_BP/DifferenceTick.DifferenceTick_C|GetIsFound _asdifference_tick))
            (Default|ShowDiff _asdifference_tick)))
        (:CastFailed
          (bind _returnvalue_2 (UserInterface|CreateWidget "/Game/_Widgets/GameOver.GameOver_C" self))
          (UserInterface|Viewport|AddtoViewport _returnvalue_2 0)
          (Game|SetGamePaused true))))))

(fn ConstructionScript)