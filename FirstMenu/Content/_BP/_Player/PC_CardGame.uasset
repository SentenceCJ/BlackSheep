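; Player controller for a memory pair-matching card game, handling card picking, match checks and completion.
; Interact line-traces under the mouse and flips an unrotated BP_Card, storing up to two picks before a delayed comparison.
; Mismatches flip back and subtract time from the game instance's Timer.
; Matches count toward a pair total derived from the level's card count, pausing the game once all are found.
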(event Custom|CompareCards
  (bind _currentpairs (Variables|Default|GetcurrentPairs))
  (if (and (Utilities|IsValid (Variables|Default|GetfirstCard)) (Utilities|IsValid (Variables|Default|GetsecondCard)))
    (if (== (Variables|/Game/_BP/BP_Card.BP_Card_C|GetCardNumber (Variables|Default|GetfirstCard)) (Variables|/Game/_BP/BP_Card.BP_Card_C|GetCardNumber (Variables|Default|GetsecondCard)))
      (Variables|Default|SetfirstCard 0)
      (Variables|Default|SetsecondCard 0)
      (Math|Integer|IncrementInt _currentpairs
        (:%20%20
          (if (== _currentpairs (Variables|Default|GettotalPairs))
            (Utilities|FlowControl|Delay 1.0)
            (Game|SetGamePaused true))))
      (else
        (Default|ReverseCardRotation (Variables|Default|GetfirstCard))
        (Default|ReverseCardRotation (Variables|Default|GetsecondCard))
        (Variables|Default|SetfirstCard 0)
        (Variables|Default|SetsecondCard 0)
        (CallFunction|RemoveTImer)))))

(event Custom|RemoveTImer
  (bind _asbp_game_instance (Utilities|Casting|CastToBP_GameInstance (Game|GetGameInstance)))
  (Variables|/Game/_BP/BP_GameInstance.BP_GameInstance_C|Settimer _asbp_game_instance (- (Variables|/Game/_BP/BP_GameInstance.BP_GameInstance_C|Gettimer _asbp_game_instance) 5.0)))

(event EventBeginPlay
  (bind _outactors (Actor|GetAllActorsOfClass "/Game/_BP/BP_Card.BP_Card_C"))
  (Variables|Default|SettotalPairs (/ (Utilities|Array|Length _outactors) 2)))

(event Input|ActionEvents|InputActionInteract
  (params (Key :type Key%20Structure :default "None"))
  (bind (_worldlocation _worlddirection) (Game|Player|ConvertMouseLocationToWorldSpace))
  (:Pressed
    (if (Math|Boolean|NANDBoolean (Utilities|IsValid (Variables|Default|GetfirstCard)) (Utilities|IsValid (Variables|Default|GetsecondCard)))
      (bind (_outhit _returnvalue) (Collision|LineTraceByChannel _worldlocation (+ _worldlocation (* _worlddirection 1.5e+03)) "TraceTypeQuery1" false 0 "None"))
      (if _returnvalue
        (bind _asbp_card (Utilities|Casting|CastToBP_Card (.HitActor (Collision|BreakHitResult _outhit))))
        (if (not (Variables|/Game/_BP/BP_Card.BP_Card_C|GetbRotated _asbp_card))
          (Default|Rotatecard _asbp_card)
          (Utilities|IsValid (Variables|Default|GetfirstCard)
            (:Is%20Valid
              (Variables|Default|SetsecondCard _asbp_card)
              (Utilities|FlowControl|Delay 1.0)
              (CallFunction|CompareCards))
            (:Is%20Not%20Valid
              (Variables|Default|SetfirstCard _asbp_card))))))))

(fn ConstructionScript)