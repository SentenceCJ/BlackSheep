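; BP_Door is a door that toggles open and closed, with an optional lockpick setup when it starts locked.
; On BeginPlay, a locked door picks a random lockpick range start and derives the end from a Difficulty-based width, narrower at harder levels.
; OpenDoor flips Opened and plays or reverses a timeline that eases the door's yaw with SinusoidalOut.
; OpenDoor itself does not check the locked state.
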(event Custom|Open%20Door
  (bind _door (Variables|Default|GetDoor))
  (bind _relativerotation (Variables|/Script/Engine.SceneComponent|GetRelativeRotation _door))
  (if (not (Variables|Default|Getopened?))
    (Variables|Default|Setopened? true)
    (bind _lerp (Timeline|Timeline_0 Play)
      (:Update
        (Transformation|SetRelativeRotation _door (Math|Rotator|MakeRotator (.roll _relativerotation) (.pitch _relativerotation) (Math|Interpolation|Ease "SinusoidalOut" _lerp 0.0 9e+01)) false false)))
    (else
      (Variables|Default|Setopened? false)
      (Timeline|Timeline_0 Reverse))))

(event EventBeginPlay
  (if (Variables|Default|GetLockedState)
    (Utilities|Array|SetArrayElem (Variables|Default|GetLockpick%20Range) 0 (Math|Random|RandomFloatinRange 0.0 1.6e+02))
    (Utilities|Array|SetArrayElem (Variables|Default|GetLockpick%20Range) 1 (+ (Utilities|Array|Get(acopy) (Variables|Default|GetLockpick%20Range)) (Utilities|Select :Index (Variables|Default|GetDifficulty) :NewEnumerator0 2e+01 :NewEnumerator1 15.0 :NewEnumerator2 1e+01 :NewEnumerator3 5.0)))))

(fn ConstructionScript)